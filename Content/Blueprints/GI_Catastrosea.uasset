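; GI_Catastrosea is the game instance for Catastrosea, fetching the player's account profile from a web backend.
; GetUserInformation sends a VaRest GET request to a URL built from the base address, info page and user key.
; It parses the response fields into variables for online status, identity, ban state, player stats and fleet, converting numeric stats from strings to integers.
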(event `GetUserInformation`
  ;[1 1 1] Get User Information
  (bind _result (`VaRestRequestJSON.ApplyURL` (`VaRestRequestJSON.ConstructRequestExt` "GET" "x_www_form_urlencoded_url") (`KismetStringLibrary.Concat_StrStr` (`self.URL`) (`self.InfoPage`) "?rk=" (`self.UserKey`) (`self.FName`) "userinfo")))
  (set `self.B_Status` (`KismetStringLibrary.EqualEqual_StrStr` (`VaRestJsonValue.AsString` (`VaRestJsonObject.GetField` _result "status")) "online"))
  (set `self.Username` (`VaRestJsonValue.AsString` (`VaRestJsonObject.GetField` _result "username")))
  (set `self.Email` (`VaRestJsonValue.AsString` (`VaRestJsonObject.GetField` _result "email")))
  (set `self.Banned` (`VaRestJsonValue.AsString` (`VaRestJsonObject.GetField` _result "banned")))
  (set `self.Kills` (`KismetStringLibrary.Conv_StringToInt` (`VaRestJsonValue.AsString` (`VaRestJsonObject.GetField` _result "kills"))))
  (set `self.Reputation` (`KismetStringLibrary.Conv_StringToInt` (`VaRestJsonValue.AsString` (`VaRestJsonObject.GetField` _result "reputation"))))
  (set `self.Gold` (`KismetStringLibrary.Conv_StringToInt` (`VaRestJsonValue.AsString` (`VaRestJsonObject.GetField` _result "gold"))))
  (set `self.Fleet` (`VaRestJsonValue.AsString` (`VaRestJsonObject.GetField` _result "fleet"))))