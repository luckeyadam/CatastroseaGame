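; PlayerPawn is the player's Blueprint, adding physics object pickup, vertical swim input and a local HUD.
; On BeginPlay it shows crosshair and health bar widgets for the locally controlled player only.
; F toggles between grabbing a simulating object found by a short camera line trace and releasing it, with a Physics Handle pulling it to HeldObjectLocation every tick.
; The MoveUP axis adds vertical movement only while swimming.
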(event `self.ReceiveBeginPlay`
  ;[1 1 1] UI
  (if (`self.IsLocallyControlled`)
    (bind _returnvalue (`|CreateWidget` "/Game/UI/WBP_Crosshair.WBP_Crosshair_C"))
    (`UserWidget.AddToViewport` _returnvalue 0)
    (bind _returnvalue_2 (`|CreateWidget` "/Game/UI/WBP_HealthBar.WBP_HealthBar_C"))
    (bind _output_get (set `self.HealthBarRef` _returnvalue_2))
    (`UserWidget.AddToViewport` _output_get 0)))

(event `self.ReceiveTick`
  (params (DeltaSeconds :type "Float (single-precision)"))
  (`PhysicsHandleComponent.SetTargetLocation` (`self.PhysicsHandle`) (`SceneComponent.K2_GetComponentLocation` (`self.HeldObjectLocation`))))

(event `PickupObject`
  (bind _cameracomp (`self.CameraComp`))
  (bind _returnvalue (`SceneComponent.K2_GetComponentLocation` _cameracomp))
  ;[1 1 1] Pick Up Objects
  (bind (_outhit _returnvalue_2) (`KismetSystemLibrary.LineTraceSingle` :`Start` _returnvalue :`End` (+ (* (`SceneComponent.GetForwardVector` _cameracomp) 300.0) _returnvalue) :`TraceChannel` "TraceTypeQuery1" :`DrawDebugType` "ForDuration"))
  (if _returnvalue_2
    (bind (_bblockinghit _binitialoverlap _time _distance _location _impactpoint _normal _impactnormal _physmat _hitactor _hitcomponent) (`GameplayStatics.BreakHitResult` _outhit))
    (if (`SceneComponent.IsSimulatingPhysics` _hitcomponent "None")
      (`PhysicsHandleComponent.GrabComponentAtLocation` (`self.PhysicsHandle`) _hitcomponent "None" (`SceneComponent.K2_GetComponentLocation` _hitcomponent))
      (set `self.IsHoldingObject` true))))

(event `Key|F`
  (params (Key :type "Key Structure"))
  ;[1 1 1] Pick Up Objects
  (:`Pressed`
    (if (`self.IsHoldingObject`)
      (`self.DropObject`)
      (else
        (`self.PickupObject`)))))

(event `DropObject`
  ;[1 1 1] Pick Up Objects
  (`PhysicsHandleComponent.ReleaseComponent` (`self.PhysicsHandle`))
  (set `self.IsHoldingObject` false))

(event `InputAxis|MoveUP`
  (params (AxisValue :type "Float (single-precision)"))
  ;[1 1 1] Swimming
  (if (`NavMovementComponent.IsSwimming` (`self.CharacterMovement`))
    (`self.AddMovementInput` (`KismetMathLibrary.GetUpVector` (`KismetMathLibrary.MakeRotator` 0.0 0.0 (.yaw (`self.GetControlRotation`)))) AxisValue)))

(fn `UserConstructionScript`)