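; Game mode for Catastrosea that holds logic to spawn sea mines at locations found by an environment query.
; On query success, it draws a debug sphere at each result, spawns a BP_SeaMine there with collision adjustment and prints its name.
; The EQS_FindSpawnLocation query call and its callback binding are not connected to any event, and SpawnNewBot is empty, so no spawning is triggered here.
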(event `self.SpawnNewBot`)

(event `OnQueryFinishedEvent_Event_0`
  (params (QueryInstance :type "EnvQueryInstanceBlueprintWrapper Object Reference") (QueryStatus :type "EEnvQueryStatus Enum" :default "Processing"))
  (switch `EEnvQueryStatus` QueryStatus
    (:`Success`
      (for _array_element (`EnvQueryInstanceBlueprintWrapper.GetResultsAsLocations` QueryInstance)
        (`KismetSystemLibrary.DrawDebugSphere` _array_element 50.0 12 (struct :`R` 0.854167 :`G` 0.835445 :`B` 0.05151 :`A` 1.0) 2.0 2.0)
        (bind _returnvalue (`|SpawnActorFromClass` "/Game/SeaMine/BP_SeaMine.BP_SeaMine_C" (`KismetMathLibrary.MakeTransform` _array_element) "AdjustIfPossibleButDontSpawnIfColliding" "OverrideRootScale" null null))
        (`KismetSystemLibrary.PrintString` (`KismetSystemLibrary.GetDisplayName` _returnvalue))))))

(fn `UserConstructionScript`)